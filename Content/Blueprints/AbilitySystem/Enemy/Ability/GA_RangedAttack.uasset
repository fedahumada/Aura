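; Enemy ranged attack gameplay ability that fires a projectile at the avatar's combat target.
; On activation it turns the avatar toward the target through interface messages, then plays a random tagged attack montage.
; A gameplay event wait spawns the projectile at the target's current location and ends the ability, as does montage completion, interruption or cancellation.
; The montage and event tag come from separate random picks, so they can differ.
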(event Ability|EventActivateAbility
  (bind _output_get (Variables|Default|SetAvatarActorInfo (Ability|GetAvatarActorfromActorInfo)))
  (bind _returnvalue (Class|EnemyInterface|GetCombatTarget(Message) _output_get))
  (Class|CombatInterface|UpdateFacingTarget(Message) (Variables|Default|GetAvatarActorInfo) (Transformation|GetActorLocation _returnvalue))
  (bind _returnvalue_2 (Class|CombatInterface|GetAttackMontages(Message) (Variables|Default|GetAvatarActorInfo)))
  (|PlayMontageandWaitProxy "None" (.montage (Class|AuraDamageGameplayAbility|GetRandomTaggedMontagefromArray _returnvalue_2)) 1.0 "None" true 1.0 0.0 false
    (:then
      (Ability|Tasks|WaitGameplayEvent (.montagetag (Class|AuraDamageGameplayAbility|GetRandomTaggedMontagefromArray _returnvalue_2)) 0
        (:EventReceived
          (bind _returnvalue_3 (Class|EnemyInterface|GetCombatTarget(Message) (Variables|Default|GetAvatarActorInfo)))
          (Class|AuraProjectileSpell|SpawnProjectile (Transformation|GetActorLocation _returnvalue_3))
          (Ability|EndAbility))))
    (:OnCompleted
      (Ability|EndAbility :!label _label))
    (:OnInterrupted
      (goto _label))
    (:OnCancelled
      (goto _label))))