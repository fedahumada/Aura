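; Gameplay ability for a melee attack against the avatar's combat target.
; On activation it passes the target's location as the facing target, then plays a randomly picked tagged attack montage.
; The montage's gameplay event triggers a small sphere query at the tag's combat socket, damaging live players found who are not friends.
; The ability ends after that hit check or when the montage completes, is interrupted or is cancelled.
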(event Ability|EventActivateAbility
  (bind _output_get (Variables|Default|SetAvatarActorInfo (Ability|GetAvatarActorfromActorInfo)))
  (bind _returnvalue (Class|EnemyInterface|GetCombatTarget(Message) _output_get))
  (Class|CombatInterface|UpdateFacingTarget(Message) (Variables|Default|GetAvatarActorInfo) (Transformation|GetActorLocation _returnvalue))
  (bind _returnvalue_2 (Class|CombatInterface|GetAttackMontages(Message) (Variables|Default|GetAvatarActorInfo)))
  (if (> (Utilities|Array|Length _returnvalue_2) 0)
    (bind _output_get_2 (Variables|Default|SetTaggedMontage (Utilities|Array|Get(acopy) _returnvalue_2 (Math|Random|RandomIntegerinRange 0 (- (Utilities|Array|Length _returnvalue_2) 1)))))
    (|PlayMontageandWaitProxy "None" (.montage _output_get_2) 1.0 "None" true 1.0 0.0 false
      (:then
        (Ability|Tasks|WaitGameplayEvent (.montagetag _output_get_2) 0
          (:EventReceived
            (bind _returnvalue_3 (Class|CombatInterface|GetCombatSocketLocation(Message) (Variables|Default|GetAvatarActorInfo) (.montagetag _output_get_2)))
            (bind _outoverlappingactors (Class|AuraAbilitySystemLibrary|GetLivePlayersWithinRadius self (Utilities|Array|MakeArray (Ability|GetAvatarActorfromActorInfo)) 45.0 _returnvalue_3))
            (for _array_element _outoverlappingactors
              (if (not (Class|AuraAbilitySystemLibrary|AreFriends (Variables|Default|GetAvatarActorInfo) _array_element))
                (Class|AuraDamageGameplayAbility|CauseDamage _array_element)
                (Ability|EndAbility)))
            (Ability|EndAbility))))
      (:OnCompleted
        (Ability|EndAbility :!label _label))
      (:OnInterrupted
        (goto _label))
      (:OnCancelled
        (goto _label)))))