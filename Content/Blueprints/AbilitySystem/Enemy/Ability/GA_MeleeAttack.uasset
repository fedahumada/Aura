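; GA_MeleeAttack is an enemy gameplay ability that turns the avatar toward its combat target and plays a random tagged attack montage.
; The montage's gameplay event triggers a small radius check at its tagged socket, damaging live non-friendly players and calling their blood effect interface.
; Any hit fires a melee impact GameplayCue carrying the montage tag.
; The ability ends after that event or when the montage completes, is interrupted or is cancelled.
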(event Ability|EventActivateAbility
  (Variables|Default|SetbHasHitTarget false)
  (bind _output_get (Variables|Default|SetAvatarActorInfo (Ability|GetAvatarActorfromActorInfo)))
  (bind _returnvalue (Class|EnemyInterface|GetCombatTarget(Message) _output_get))
  (Class|CombatInterface|UpdateFacingTarget(Message) (Variables|Default|GetAvatarActorInfo) (Transformation|GetActorLocation _returnvalue))
  (bind _returnvalue_2 (Class|CombatInterface|GetAttackMontages(Message) (Variables|Default|GetAvatarActorInfo)))
  (bind _output_get_2 (Variables|Default|SetTaggedMontage (Class|AuraDamageGameplayAbility|GetRandomTaggedMontagefromArray _returnvalue_2)))
  (|PlayMontageandWaitProxy "None" (.montage _output_get_2) 1.0 "None" true 1.0 0.0 false
    (:then
      (Ability|Tasks|WaitGameplayEvent (.montagetag (Variables|Default|GetTaggedMontage)) 0 true
        (:EventReceived
          (bind _returnvalue_3 (Class|CombatInterface|GetCombatSocketLocation(Message) (Variables|Default|GetAvatarActorInfo) (.sockettag (Variables|Default|GetTaggedMontage))))
          (bind _output_get_3 (Variables|Default|SetCombatSocketLocation _returnvalue_3))
          (bind _outoverlappingactors (Class|AuraAbilitySystemLibrary|GetLivePlayersWithinRadius self (Utilities|Array|MakeArray (Ability|GetAvatarActorfromActorInfo)) 45.0 _output_get_3))
          (for _array_element _outoverlappingactors
            (if (not (Class|AuraAbilitySystemLibrary|AreFriends (Variables|Default|GetAvatarActorInfo) _array_element))
              (Class|AuraDamageGameplayAbility|CauseDamage _array_element)
              (Variables|Default|SetbHasHitTarget true)
              (Class|CombatInterface|GetBloodEffect(Message) _array_element)))
          (if (Variables|Default|GetbHasHitTarget)
            (bind _returnvalue_4 (Class|EnemyInterface|GetCombatTarget(Message) (Variables|Default|GetAvatarActorInfo)))
            (Class|GameplayAbility|ExecuteGameplayCuewithParams "(TagName=\"GameplayCue.MeleeImpact\")" (Ability|GameplayCue|MakeGameplayCueParameters :AggregatedSourceTags (GameplayTags|MakeGameplayTagContainerfromTag (.montagetag (Variables|Default|GetTaggedMontage))) :Location (Variables|Default|GetCombatSocketLocation) :SourceObject _returnvalue_4)))
          (Ability|EndAbility))))
    (:OnCompleted
      (Ability|EndAbility :!label _label))
    (:OnInterrupted
      (goto _label))
    (:OnCancelled
      (goto _label))))