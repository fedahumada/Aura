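; BP_FlamePillar is a flame pillar actor whose FireLight flickers continuously.
; From BeginPlay, it randomly picks one of two intensity timelines, and each picks again when it finishes, forming an endless, varied loop.
; Timeline updates feed ScaleFlameIntensity, which offsets the curve value and scales it by a fraction of BaseIntensity to set the light's intensity.
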(event Custom|ChooseTimeLine
  ;[1 1 1] SetFlameIntensity
  (switch int (Math|Random|RandomIntegerinRange 0 1)
    (:Default
      (CallFunction|StartTimeline1))
    (:0
      (CallFunction|StartTimeline1))
    (:1
      (CallFunction|StartTimeline2))))

(event Custom|StartTimeline_2
  ;[1 1 1] SetFlameIntensity
  (bind _intensity (Timeline|FlameIntensity_2 PlayFromStart)
    (:Update
      (CallFunction|ScaleFlameIntensity _intensity))
    (:Finished
      (CallFunction|ChooseTimeLine))))

(event Custom|StartTimeline_1
  ;[1 1 1] SetFlameIntensity
  (bind _intensity (Timeline|FlameIntensity_1 PlayFromStart)
    (:Update
      (CallFunction|ScaleFlameIntensity _intensity))
    (:Finished
      (CallFunction|ChooseTimeLine))))

(event EventBeginPlay
  ;[1 1 1] SetFlameIntensity
  (CallFunction|ChooseTimeLine))

(fn ConstructionScript)

(fn ScaleFlameIntensity
  (params (Intensity :type Float%20%28double-precision%29))
  (Rendering|Components|Light|SetIntensity (Variables|Default|GetFireLight) (* (+ Intensity -0.5) (* 0.2 (Variables|Default|GetBaseIntensity)))))